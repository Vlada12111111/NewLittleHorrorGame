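; BP_Pedestal is a StoneQuest pedestal that receives a stone actor and lights up.
; PutStone stores the actor in BPStone, moves it to the Scene component's world location and shows the SpotLight.
; It also flips the boolean NewVar, though both branches turn the light on, so nothing here switches it off.
; The Take function is an empty stub.
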(event `/Game/Bluprints/StoneQuest/PickUpStones.PutStone`
  (params (Actor :type "/Game/Bluprints/StoneQuest/BP_QuestSymbolStone Object Reference"))
  (bind _output_get (set `self.BP_Stone` Actor))
  (`self.K2_SetActorLocation` _output_get (`SceneComponent.K2_GetComponentLocation` (`self.Scene`)) false false)
  (if (`self.NewVar`)
    (`SceneComponent.SetVisibility` (`self.SpotLight`) true false)
    (set `self.NewVar` false)
    (else
      (`SceneComponent.SetVisibility` (`self.SpotLight`) true false)
      (set `self.NewVar` true))))

(fn `Take`
  (returns (Actor :type "/Game/Bluprints/StoneQuest/BP_QuestSymbolStone Object Reference"))
  (return null))

(fn `UserConstructionScript`)