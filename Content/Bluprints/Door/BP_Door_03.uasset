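; Door Blueprint that toggles open and closed and shows an outline and prompt widget when focused.
; ChengeDoorStatus flip-flops a timeline forward and back to set the mesh's yaw, with paired DoOnce gates alternating open and close sounds played at world origin.
; OnFocus optionally enables custom depth for the outline and creates the widget once, while a short retriggerable delay clears both when focus calls stop.
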(event `/Game/Bluprints/Door/BPI_Interact.ChengeDoorStatus`
  ;[1 1 1] Open Door
  (`/Engine/EditorBlueprintResources/StandardMacros.FlipFlop`
    (:`A`
      (`|ExecutionSequence`
        (:`then_0`
          (`/Engine/EditorBlueprintResources/StandardMacros.DoOnce` false :!label _label
            (:`Completed`
              (`GameplayStatics.PlaySoundAtLocation` "/Game/Asets/VHExterior/Audio/Cues/Cue_OpenDoor_01.Cue_OpenDoor_01" (0.0 0.0 0.0) (struct) 1.0 1.0 0.0 null null null null)
              (goto _label_3 :!via `Reset`))))
        (:`then_1`
          (bind (_direction _doorrotater) (`Timeline|Door` :!label _label_2)
            (:`Update`
              (`SceneComponent.K2_SetRelativeRotation` (`self.Mesh_Door_02`) (`KismetMathLibrary.MakeRotator` 0.0 0.0 _doorrotater) false false))))))
    (:`B`
      (`|ExecutionSequence`
        (:`then_0`
          (goto _label_2 :!via `Reverse`))
        (:`then_1`
          (`/Engine/EditorBlueprintResources/StandardMacros.DoOnce` false :!label _label_3
            (:`Completed`
              (`GameplayStatics.PlaySoundAtLocation` "/Game/Asets/VHExterior/Audio/Cues/Cue_CloseDoor_01.Cue_CloseDoor_01" (0.0 0.0 0.0) (struct) 1.0 1.0 0.0 null null null null)
              (goto _label :!via `Reset`))))))))

(event `/Game/Asets/VHExterior/Blueprints/BP_InteractInterface.On Focus`
  ;[1 1 1] Outline
  (`|ExecutionSequence`
    (:`then_0`
      (if (`self.Outline on/off`)
        (`self.BeginFocus`))
      (set `self.TimeOutlineEnd` 0.1)
      (`KismetSystemLibrary.RetriggerableDelay` (`self.TimeOutlineEnd`))
      (`self.EndFocus`)
      (`Widget.RemoveFromParent` (stale _returnvalue))
      (`self.Reset` false))
    (:`then_1`
      (`/Engine/EditorBlueprintResources/StandardMacros.Do N` 1 :!label _label_4
        (:`Exit`
          (bind _returnvalue (`|CreateWidget` "/Game/Asets/VHExterior/UMG/Door_Widget.Door_Widget_C"))
          (`UserWidget.AddToViewport` _returnvalue 0))))))

(event `Reset`
  (params (NewParam :type Boolean))
  ;[1 1 1] Outline
  (goto _label_4 :!via `Reset`))

(fn `BeginFocus`
  (`PrimitiveComponent.SetRenderCustomDepth` (`self.Mesh_Door_02`) true))

(fn `EndFocus`
  (`PrimitiveComponent.SetRenderCustomDepth` (`self.Mesh_Door_02`) false))

(fn `UserConstructionScript`)