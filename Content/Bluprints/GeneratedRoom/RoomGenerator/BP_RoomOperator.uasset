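; Room operator for generated rooms that scores room-class similarity, picks replacements and manages the layout's connection graph.
; CompareRoom scores size, doors, type and furniture placement, but its return is unwired, so CompareMatrix receives no real scores.
; The matrix is cached in a SaveGame, rebuilt on room-count mismatch, and drives randomized replacement by normalized score.
; RoomConnector serves as an adjacency matrix for recursive branch-size counting, corner checks and room removal.
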(fn `CompareFloat`
  (params (CompareRoom1 :type "Float (double-precision)") (CompareRoom2 :type "Float (double-precision)"))
  (returns (Result :type "Float (double-precision)"))
  (return (/ (`KismetMathLibrary.FMin` CompareRoom1 CompareRoom2) (`KismetMathLibrary.FMax` CompareRoom1 CompareRoom2))))

(fn `CompareFurniture`
  (params (Object1 :type "Array of StaticMesh Soft Object Reference") (Position1 :type "Array of Vector Structure") (Object2 :type "Array of StaticMesh Soft Object Reference") (Position2 :type "Array of Vector Structure"))
  (returns (Result :type "Float (double-precision)"))
  (locals (SummaryResult :type "Float (double-precision)") (Pos1 :type "Array of Vector Structure") (Pos2 :type "Array of Vector Structure"))
  ;[1 1 1] Используются циклы для перебора элементов массивов и проверка условий где результат возвращается через Return Node.
  ;;[1 1 1] Input / seve Data
  (set `local.Pos1` Position1)
  (set `local.Pos2` Position2)
  (`|ExecutionSequence`
    (:`then_0`
      ;;[1 1 1] Get item 1
      (for (_array_element _array_index) Object1
        (if (`KismetArrayLibrary.Array_Contains` Object2 _array_element)
          ;;[1 1 1] Get item 2
          (for (_array_element_2 _array_index_2) Object2
            (if (== _array_element _array_element_2)
              (bind _returnvalue (`KismetMathLibrary.Vector_Distance` (`|GetArrayItem` (`local.Pos1`) _array_index) (`|GetArrayItem` (`local.Pos2`) _array_index_2)))
              ;;[1 1 1] verify distance
              (if (< _returnvalue 3.0)
                ;;[1 1 1] Calculate item Compares
                (set `local.SummaryResult` (+ (`local.SummaryResult`) (`KismetMathLibrary.FClamp` (- 1.0 (/ _returnvalue 3.0)) 0.5)))
                (else
                  (set `local.SummaryResult` (+ (`local.SummaryResult`) 0.5)))))))))
    (:`then_1`
      ;;[1 1 1] Return Result
      (return (/ (`local.SummaryResult`) (`KismetMathLibrary.Max` (`KismetArrayLibrary.Array_Length` Object1) (`KismetArrayLibrary.Array_Length` Object2)))))))

(fn `CompareRoom`
  (params (roomReferences1 :type "/Game/Bluprints/GeneratedRoom/RoomGenerator/BP_Room Soft Class Reference") (roomReferences2 :type "/Game/Bluprints/GeneratedRoom/RoomGenerator/BP_Room Soft Class Reference"))
  (returns (compare :type "Float (double-precision)"))
  (locals (RoomScaleCompareResult :type "Float (double-precision)") (DoorCompareResult :type "Float (double-precision)") (room1 :type "/Game/Bluprints/GeneratedRoom/RoomGenerator/BP_Room Class Reference") (room2 :type "/Game/Bluprints/GeneratedRoom/RoomGenerator/BP_Room Class Reference") (TypeCompareResult :type Integer) (FurnitureCompareResult :type "Float (double-precision)"))
  (bind (_lenght _width _depth) (defaults `Object` (`local.room1`)))
  (bind (_lenght_2 _width_2 _depth_2) (defaults `Object` (`local.room2`)))
  (bind (_furnituremesh _furniturelokaction) (defaults `Object` (`local.room1`)))
  (bind (_furnituremesh_2 _furniturelokaction_2) (defaults `Object` (`local.room2`)))
  (`|ExecutionSequence`
    (:`then_0`
      ;[1 1 1] Loda/Save InputData
      (bind _returnvalue (`KismetSystemLibrary.LoadClassAsset_Blocking` roomReferences1))
      (bind _asbp_room (castclass `/Game/Bluprints/GeneratedRoom/RoomGenerator/BP_Room` _returnvalue))
      (set `local.room1` _asbp_room)
      (bind _returnvalue_2 (`KismetSystemLibrary.LoadClassAsset_Blocking` roomReferences2))
      (bind _asbp_room_2 (castclass `/Game/Bluprints/GeneratedRoom/RoomGenerator/BP_Room` _returnvalue_2))
      (set `local.room2` _asbp_room_2))
    (:`then_1`
      ;[1 1 1] Compare RoomScale
      ;;[1 1 1] Lenght
      (bind _result (`self.CompareFloat` _lenght_2 _lenght))
      ;;[1 1 1] Widsht
      (bind _result_2 (`self.CompareFloat` _width_2 _width))
      ;;[1 1 1] Depth
      (bind _result_3 (`self.CompareFloat` _depth_2 _depth))
      ;;[1 1 1] Calculate arange
      (set `local.RoomScaleCompareResult` (/ (+ _result _result_2 _result_3) 3.0)))
    (:`then_2`
      ;[1 1 1] Compare Door
      (bind _result_4 (`self.CompareFloat` (`KismetMathLibrary.Conv_IntToDouble` (defaults `Object` (`local.room2`))) (`KismetMathLibrary.Conv_IntToDouble` (defaults `Object` (`local.room1`)))))
      (set `local.DoorCompareResult` _result_4))
    (:`then_3`
      ;[1 1 1] Compare RoomType
      (if (`|EnumEquality` (defaults `Object` (`local.room2`)) (defaults `Object` (`local.room1`)))
        (set `local.TypeCompareResult` 1)
        (else
          (set `local.TypeCompareResult` 0))))
    (:`then_4`
      ;[1 1 1] CompareFurniture
      (bind _result_5 (`self.CompareFurniture` _furnituremesh _furniturelokaction _furnituremesh_2 _furniturelokaction_2))
      (set `local.FurnitureCompareResult` _result_5))))

(fn `GeneratorCampare`
  (for (_array_element _array_index) (`self.Room`)
    (for (_array_element_2 _array_index_2) (`self.Room`)
      (if (== _array_element _array_element_2)
        (`KismetArrayLibrary.Array_Set` (`.SubArray_4_18DD20634C6623534ECCAB946D3A8BB9` (break `/Game/Bluprints/GeneratedRoom/RoomGenerator/2Daray` (`|GetArrayItem` (`self.CompareMatrix`) _array_index))) _array_index_2 -1.0)
        (else
          (bind _compare (`self.CompareRoom` _array_element_2 _array_element))
          (`KismetArrayLibrary.Array_Set` (`.SubArray_4_18DD20634C6623534ECCAB946D3A8BB9` (break `/Game/Bluprints/GeneratedRoom/RoomGenerator/2Daray` (`|GetArrayItem` (`self.CompareMatrix`) _array_index))) _array_index_2 _compare))))))

(fn `IsCorner`
  (params (InsideRoom :type "/Game/Bluprints/GeneratedRoom/RoomGenerator/BP_Room Soft Class Reference") (OutRoom :type "/Game/Bluprints/GeneratedRoom/RoomGenerator/BP_Room Soft Class Reference") (Lenght :type Integer))
  (returns (Result :type Boolean))
  (bind _doornumber (`self.QuantityRoomNumber` InsideRoom OutRoom))
  (return (<= _doornumber Lenght)))

(fn `LoadMemoryGame`
  (bind _returnvalue (`GameplayStatics.DoesSaveGameExist` (`self.MemorySlot`)))
  (if _returnvalue
    (bind _returnvalue_2 (`GameplayStatics.LoadGameFromSlot` (`self.MemorySlot`)))
    (bind _asmatrix (cast `/Game/Bluprints/GeneratedRoom/RoomGenerator/Matrix` _returnvalue_2))
    (bind _matrix2derey (`/Game/Bluprints/GeneratedRoom/RoomGenerator/Matrix.Matrix2Derey` _asmatrix))
    (if (== (`KismetArrayLibrary.Array_Length` _matrix2derey) (`KismetArrayLibrary.Array_Length` (`self.Room`)))
      (set `self.CompareMatrix` _matrix2derey)
      (else
        (`self.GeneratorCampare`)
        (`self.SaveMemory`)))
    (else
      (`self.GeneratorCampare`)
      (`self.SaveMemory`))))

(fn `QuantityRoomNumber`
  (params (InsideRoom :type "/Game/Bluprints/GeneratedRoom/RoomGenerator/BP_Room Soft Class Reference") (OutRoom :type "/Game/Bluprints/GeneratedRoom/RoomGenerator/BP_Room Soft Class Reference"))
  (returns (DoorNumber :type Integer))
  (locals (RoomNum :type Integer))
  (bind _roomuse (`self.RoomUse`))
  (bind _subarray (break `/Game/Bluprints/GeneratedRoom/RoomGenerator/2Daray` (`|GetArrayItem` (`self.RoomConnector`) (`KismetArrayLibrary.Array_Find` _roomuse OutRoom))))
  (for _array_element _subarray
    (if (== _array_element 1.0)
      (`/Engine/EditorBlueprintResources/StandardMacros.IncrementInt` (`local.RoomNum`))))
  (if (== (`local.RoomNum`) 1)
    (return 1)
    (else
      (set `local.RoomNum` 1)
      (for (_array_element_2 _array_index) _subarray
        (if (and (== _array_element_2 1.0) (!= _array_index (`KismetArrayLibrary.Array_Find` _roomuse InsideRoom)))
          (bind _doornumber (`self.QuantityRoomNumber` InsideRoom (`|GetArrayItem` (`self.RoomUse`) _array_index)))
          (set `local.RoomNum` (+ _doornumber (`local.RoomNum`)))))
      (return (`local.RoomNum`)))))

(fn `RemoveRoom`
  (params (NewParam :type "/Game/Bluprints/GeneratedRoom/RoomGenerator/BP_Room Soft Class Reference"))
  (locals (Index :type Integer))
  (set `local.Index` (`KismetArrayLibrary.Array_Find` (`self.RoomUse`) NewParam))
  (`KismetArrayLibrary.Array_RemoveItem` (`self.RoomUse`) NewParam)
  (for _array_element (`self.RoomConnector`)
    (`KismetArrayLibrary.Array_Remove` (`.SubArray_4_18DD20634C6623534ECCAB946D3A8BB9` (break `/Game/Bluprints/GeneratedRoom/RoomGenerator/2Daray` _array_element)) (`local.Index`)))
  (`KismetArrayLibrary.Array_Remove` (`self.RoomConnector`) (`local.Index`)))

(fn `ReplacementOfRooms`
  (params (OldRoom :type "/Game/Bluprints/GeneratedRoom/RoomGenerator/BP_Room Soft Class Reference"))
  (returns (NewRoom :type "/Game/Bluprints/GeneratedRoom/RoomGenerator/BP_Room Soft Class Reference"))
  (locals (CompareSum :type "Float (double-precision)") (ChangesPercentage :type "Array of Float (double-precision)"))
  (bind _subarray (break `/Game/Bluprints/GeneratedRoom/RoomGenerator/2Daray` (`|GetArrayItem` (`self.CompareMatrix`) (`KismetArrayLibrary.Array_Find` (`self.Room`) OldRoom))))
  ;[1 1 1] ConformityRoom
  ;[1 1 1] FoundSum
  (for _array_element _subarray
    (set `local.CompareSum` (+ _array_element (`local.CompareSum`))))
  ;[1 1 1] FoundPercentageRoom
  (for (_array_element_2 _array_index) _subarray
    (`KismetArrayLibrary.Array_Set` (`local.ChangesPercentage`) _array_index (/ _array_element_2 (`local.CompareSum`))))
  ;[1 1 1] Randomizer
  (for (_array_element_3 _array_index_2) (`local.ChangesPercentage`)
    (if (>= _array_element_3 (`KismetMathLibrary.RandomFloat`))
      (return (`|GetArrayItem` (`self.Room`) _array_index_2))))
  (return (`KismetArrayLibrary.Array_Random` (`self.Room`))))

(fn `SaveMemory`
  (locals (SaveObject :type "/Game/Bluprints/GeneratedRoom/RoomGenerator/Matrix Object Reference"))
  (bind _returnvalue (`GameplayStatics.DoesSaveGameExist` (`self.MemorySlot`)))
  (if _returnvalue
    (bind _returnvalue_2 (`GameplayStatics.LoadGameFromSlot` (`self.MemorySlot`)))
    (bind _asmatrix (cast `/Game/Bluprints/GeneratedRoom/RoomGenerator/Matrix` _returnvalue_2))
    (set `local.SaveObject` _asmatrix)
    (else
      (bind _returnvalue_3 (`GameplayStatics.CreateSaveGameObject` "/Game/Bluprints/GeneratedRoom/RoomGenerator/Matrix.Matrix_C"))
      (set `local.SaveObject` _returnvalue_3)))
  (set `/Game/Bluprints/GeneratedRoom/RoomGenerator/Matrix.Matrix2Derey` (`self.CompareMatrix`) (`local.SaveObject`))
  (`GameplayStatics.SaveGameToSlot` (`local.SaveObject`) (`self.MemorySlot`)))

(fn `UserConstructionScript`)