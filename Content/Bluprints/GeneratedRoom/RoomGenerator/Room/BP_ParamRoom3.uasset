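; BP_ParamRoom3 is a room Blueprint under the RoomGenerator folder that registers two door points.
; Its Construction Script runs the parent's script, then casts two Child Actor components to BP_PointDoor and appends each to DoorReference.
; The casts are chained, so a failed cast stops any later registration.
; The event graph holds only disabled default events, so it adds no runtime logic of its own.
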(fn `UserConstructionScript`
  (`parent.UserConstructionScript`)
  (bind _asbp_point_door_ (cast `/Game/Bluprints/GeneratedRoom/RoomGenerator/BP_PointDoor` (`ChildActorComponent.ChildActor` (`self.ChildActor`))))
  (`KismetArrayLibrary.Array_Add` (`self.DoorReference`) _asbp_point_door_)
  (bind _asbp_point_door__2 (cast `/Game/Bluprints/GeneratedRoom/RoomGenerator/BP_PointDoor` (`ChildActorComponent.ChildActor` (`self.ChildActor2`))))
  (`KismetArrayLibrary.Array_Add` (`self.DoorReference`) _asbp_point_door__2))