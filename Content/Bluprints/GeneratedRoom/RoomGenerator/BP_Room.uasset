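; BP_Room is a room actor in the room generator that reports when the player walks into it.
; On BeginPlay it stores the world scale of its RoomSize component as Lenght, Width and Depth.
; When the player pawn overlaps RoomSize, it finds BP_RoomOperator with GetActorOfClass and calls PlayerWalkInRoom, passing the room's class rather than the instance.
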(event `self.ReceiveBeginPlay`
  (set `self.Lenght` (.x (`SceneComponent.K2_GetComponentScale` (`self.RoomSize`))))
  (set `self.Width` (.y (`SceneComponent.K2_GetComponentScale` (`self.RoomSize`))))
  (set `self.Depth` (.z (`SceneComponent.K2_GetComponentScale` (`self.RoomSize`)))))

(event `self.RoomSize.OnComponentBeginOverlap`
  (params (OverlappedComponent :type "PrimitiveComponent Object Reference") (OtherActor :type "Actor Object Reference") (OtherComp :type "PrimitiveComponent Object Reference") (OtherBodyIndex :type Integer) (bFromSweep :type Boolean) (SweepResult :type "HitResult Structure (by ref)"))
  (if (== OtherActor (`GameplayStatics.GetPlayerPawn` 0))
    (bind _returnvalue (`GameplayStatics.GetActorOfClass` "/Game/Bluprints/GeneratedRoom/RoomGenerator/BP_RoomOperator.BP_RoomOperator_C"))
    (`/Game/Bluprints/GeneratedRoom/RoomGenerator/BP_RoomOperator.PlayerWalkInRoom` _returnvalue (`|ConvertAsset` (`GameplayStatics.GetObjectClass` self)))))

(fn `UserConstructionScript`)