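; BP_Room9 is a room Blueprint for the room generator, with two door points placed as child actors.
; Its Construction Script runs the parent script, casts both child actors to BP_PointDoor and adds them to the DoorRef array.
; Both casts run before either add, so one failed cast leaves both doors unregistered.
; The Event Graph holds only disabled placeholder events.
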(fn `UserConstructionScript`
  (`parent.UserConstructionScript`)
  (bind _asbp_point_door (cast `/Game/Bluprints/GeneratedRoom/RoomGenerator/BP_PointDoor` (`ChildActorComponent.ChildActor` (`self.ChildActor`))))
  (bind _asbp_point_door_2 (cast `/Game/Bluprints/GeneratedRoom/RoomGenerator/BP_PointDoor` (`ChildActorComponent.ChildActor` (`self.ChildActor1`))))
  (`KismetArrayLibrary.Array_Add` (`self.DoorRef`) _asbp_point_door)
  (`KismetArrayLibrary.Array_Add` (`self.DoorRef`) _asbp_point_door_2))