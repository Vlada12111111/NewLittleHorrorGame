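; BP_Candle2 is a candle light that toggles on and off through its ChangeLiting event.
; A FlipFlop alternates the visibility of four planes and two point lights, with the first call switching them off at once.
; Switching on follows a half-second delay, and each change plays the CandleOn or CandleOff sound at the world origin rather than at the candle.
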(event `/Game/Bluprints/LightHome/Candle/BPI_Candle.ChangeLiting`
  ;[1 1 1] On/Off Light
  (`/Engine/EditorBlueprintResources/StandardMacros.FlipFlop`
    (:`A`
      (`SceneComponent.SetVisibility` (`self.Plane1`) false false)
      (`SceneComponent.SetVisibility` (`self.Plane`) false false)
      (`SceneComponent.SetVisibility` (`self.Plane2`) false false)
      (`SceneComponent.SetVisibility` (`self.Plane3`) false false)
      (`SceneComponent.SetVisibility` (`self.PointLight`) false false)
      (`SceneComponent.SetVisibility` (`self.PointLight1`) false false)
      (`GameplayStatics.PlaySoundAtLocation` "/Game/Bluprints/LightHome/Candle/CandleOff.CandleOff" (0.0 0.0 0.0) (struct) 1.0 1.0 0.0 null null null null))
    (:`B`
      (`KismetSystemLibrary.Delay` 0.5)
      (`SceneComponent.SetVisibility` (`self.Plane1`) true false)
      (`SceneComponent.SetVisibility` (`self.Plane`) true false)
      (`SceneComponent.SetVisibility` (`self.Plane2`) true false)
      (`SceneComponent.SetVisibility` (`self.Plane3`) true false)
      (`SceneComponent.SetVisibility` (`self.PointLight`) true false)
      (`SceneComponent.SetVisibility` (`self.PointLight1`) true false)
      (`GameplayStatics.PlaySoundAtLocation` "/Game/Bluprints/LightHome/Candle/CandleOn.CandleOn" (0.0 0.0 0.0) (struct) 1.0 1.0 0.0 null null null null))))

(fn `UserConstructionScript`)