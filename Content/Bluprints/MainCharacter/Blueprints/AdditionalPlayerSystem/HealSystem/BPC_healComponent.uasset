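; Health component that tracks the owner's HP, regenerates it after damage and shows blood screen feedback.
; GetDamage subtracts HP and destroys the owner when it equals exactly zero; otherwise it starts healing and adds a random blood screen widget, loaded synchronously, to the viewport.
; StartHeal waits a set delay, adds one HP and re-calls itself until MaxHP, with a flag blocking overlapping heal loops.
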(event `self.ReceiveBeginPlay`
  (set `self.HP` (`self.MaxHP`)))

(event `GetDamage`
  (params (damage :type Integer))
  (bind _bloodscreen (`self.BloodScreen`))
  (bind _output_get (set `self.HP` (- (`self.HP`) damage)))
  (if (== _output_get 0)
    (`Actor.K2_DestroyActor` (`self.GetOwner` self))
    (else
      (`self.StartHeal`)
      (bind _returnvalue (`KismetSystemLibrary.LoadClassAsset_Blocking` (`|GetArrayItem` _bloodscreen (`KismetMathLibrary.RandomIntegerInRange` 0 (`KismetArrayLibrary.Array_LastIndex` _bloodscreen)))))
      (bind _asuser_widget (castclass `UserWidget` _returnvalue))
      (bind _returnvalue_2 (`|CreateWidget` _asuser_widget))
      (`UserWidget.AddToViewport` _returnvalue_2 0))))

(event `StartHeal`
  (if (not (`self.iAmHelingNow`))
    (set `self.iAmHelingNow` true)
    (`KismetSystemLibrary.Delay` (`self.HealTime`))
    (bind _result (`/Engine/EditorBlueprintResources/StandardMacros.IncrementInt` (`self.HP`))
      (:`  `
        (set `self.iAmHelingNow` false)
        (if (< _result (`self.MaxHP`))
          (`self.StartHeal`))))))