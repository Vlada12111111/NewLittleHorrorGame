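; BPC_healComponent is an actor component that tracks its owner's health and regenerates it after damage.
; HP starts at MaxHP, and GetDamage subtracts damage, destroying the owner only when HP equals exactly zero and otherwise starting healing.
; StartHeal waits HealTime, adds one point and calls itself until MaxHP is reached, with a flag blocking overlapping heal loops.
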(event `self.ReceiveBeginPlay`
  (set `self.HP` (`self.MaxHP`)))

(event `GetDamage`
  (params (damage :type Integer))
  (bind _output_get (set `self.HP` (- (`self.HP`) damage)))
  (if (== _output_get 0)
    (`Actor.K2_DestroyActor` (`self.GetOwner` self))
    (else
      (`self.StartHeal`))))

(event `StartHeal`
  (if (not (`self.iAmHelingNow`))
    (set `self.iAmHelingNow` true)
    (`KismetSystemLibrary.Delay` (`self.HealTime`))
    (bind _result (`/Engine/EditorBlueprintResources/StandardMacros.IncrementInt` (`self.HP`))
      (:`  `
        (set `self.iAmHelingNow` false)
        (if (< _result (`self.MaxHP`))
          (`self.StartHeal`))))))