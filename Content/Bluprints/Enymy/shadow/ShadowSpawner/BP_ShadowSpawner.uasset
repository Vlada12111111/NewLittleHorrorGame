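; Spawner that periodically creates BP_shadow actors at positions derived from the player's location and facing.
; A looping timer, with its random interval picked once at BeginPlay, randomly flips AngleDeg and line-traces from the player.
; The target is player position plus forward offset, rotated as a whole around world Z.
; A clear trace spawns at a similarly rotated random-distance point; a hit spawns off the surface normal if far enough from the player.
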(event `self.ReceiveBeginPlay`
  (`KismetSystemLibrary.K2_SetTimerDelegate` (delegate `SpawnShadow`) (`KismetMathLibrary.RandomFloatInRange` 1.0 10.0) true))

(event `SpawnShadow`
  (bind _returnvalue (`GameplayStatics.GetPlayerCharacter` 0))
  (bind _returnvalue_2 (`GameplayStatics.GetPlayerCharacter` 0))
  (bind _returnvalue_3 (`self.K2_GetActorLocation` _returnvalue_2))
  (if (`KismetMathLibrary.RandomBool`)
    (set `self.Angle Deg` (* (`self.Angle Deg`) -1.0)))
  (bind (_outhit _returnvalue_4) (`KismetSystemLibrary.LineTraceSingle` :`Start` _returnvalue_3 :`End` (`KismetMathLibrary.RotateAngleAxis` (+ _returnvalue_3 (* (`self.GetActorForwardVector` _returnvalue_2) (1000.0 1000.0 0.0))) (`self.Angle Deg`) (0.0 0.0 1.0)) :`TraceChannel` "TraceTypeQuery1" :`DrawDebugType` "ForDuration" :`DrawTime` 15.0))
  (if (not _returnvalue_4)
    (`|SpawnActorFromClass` "/Game/Bluprints/Enymy/shadow/Shadow/BP_shadow.BP_shadow_C" (`KismetMathLibrary.MakeTransform` (`KismetMathLibrary.RotateAngleAxis` (+ (`self.K2_GetActorLocation` _returnvalue) (* (`self.GetActorForwardVector` _returnvalue) (`KismetMathLibrary.MakeVector` (`KismetMathLibrary.RandomFloatInRange` 400.0 800.0) (`KismetMathLibrary.RandomFloatInRange` 400.0 800.0)))) (`self.Angle Deg`) (0.0 0.0 1.0))) "Undefined" "MultiplyWithRoot" null null)
    (else
      (bind (_bblockinghit _binitialoverlap _time _distance _location _impactpoint _normal) (`GameplayStatics.BreakHitResult` _outhit))
      (bind _returnvalue_5 (+ _location (* _normal (`KismetMathLibrary.RandomIntegerInRange` 150 300))))
      (if (> (`KismetMathLibrary.Vector_Distance` (`self.K2_GetActorLocation` (`GameplayStatics.GetPlayerCharacter` 0)) _returnvalue_5) 400.0)
        (`|SpawnActorFromClass` "/Game/Bluprints/Enymy/shadow/Shadow/BP_shadow.BP_shadow_C" (`KismetMathLibrary.MakeTransform` _returnvalue_5) "Undefined" "MultiplyWithRoot" null null)))))

(fn `UserConstructionScript`)