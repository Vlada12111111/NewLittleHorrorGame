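; BP_shadow is a shadow enemy that frightens and damages the player, then fades away.
; While the player is inside AggressionSphere, a self-repeating Frighten event drives the player's post-process effect in half-second cycles.
; Overlapping AttacSphere sends damage to the player, plays a sound and dissolves the shadow through an M_Fade dynamic material timeline before destroying it.
; Untouched shadows fade out similarly after a random lifetime.
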(event `self.ReceiveBeginPlay`
  (`KismetSystemLibrary.Delay` (`KismetMathLibrary.RandomFloatInRange` 25.0 35.0))
  (bind _postproces (message `/Game/Bluprints/ThirdPerson/Blueprints/Interface/BPI_GetHallucinationShader.GetPostProces` (`GameplayStatics.GetPlayerPawn` 0)))
  (set `self.PlayerPostProces` _postproces)
  (bind _returnvalue (`PrimitiveComponent.CreateDynamicMaterialInstance` (`self.Sphere`) 0 "/Game/Bluprints/Enymy/shadow/Shadow/M_Fade.M_Fade" "None"))
  (bind _output_get (set `self.destroyMat` _returnvalue))
  (`MaterialInstanceDynamic.SetScalarParameterValue` _output_get "Param" -1.0)
  (bind (_direction _newtrack_0) (`Timeline|Timeline_0`)
    (:`Update`
      (`MaterialInstanceDynamic.SetScalarParameterValue` (`self.destroyMat`) "Param" _newtrack_0))
    (:`Finished`
      (`SceneComponent.SetVisibility` (`self.PlayerPostProces`) false false)
      (`self.K2_DestroyActor`))))

(event `self.AttacSphere.OnComponentBeginOverlap`
  (params (OverlappedComponent :type "PrimitiveComponent Object Reference") (OtherActor :type "Actor Object Reference") (OtherComp :type "PrimitiveComponent Object Reference") (OtherBodyIndex :type Integer) (bFromSweep :type Boolean) (SweepResult :type "HitResult Structure (by ref)"))
  (if (== OtherActor (`GameplayStatics.GetPlayerCharacter` 0))
    (`self.Attac`)))

(event `self.AggressionSphere.OnComponentBeginOverlap`
  (params (OverlappedComponent :type "PrimitiveComponent Object Reference") (OtherActor :type "Actor Object Reference") (OtherComp :type "PrimitiveComponent Object Reference") (OtherBodyIndex :type Integer) (bFromSweep :type Boolean) (SweepResult :type "HitResult Structure (by ref)"))
  (if (== OtherActor (`GameplayStatics.GetPlayerCharacter` 0))
    (set `self.Agrecive` true)
    (bind _postproces (message `/Game/Bluprints/ThirdPerson/Blueprints/Interface/BPI_GetHallucinationShader.GetPostProces` (`GameplayStatics.GetPlayerPawn` 0)))
    (set `self.PlayerPostProces` _postproces)
    (`self.Frighten`)))

(event `self.AggressionSphere.OnComponentEndOverlap`
  (params (OverlappedComponent :type "PrimitiveComponent Object Reference") (OtherActor :type "Actor Object Reference") (OtherComp :type "PrimitiveComponent Object Reference") (OtherBodyIndex :type Integer))
  (if (== OtherActor (`GameplayStatics.GetPlayerCharacter` 0))
    (set `self.Agrecive` false)))

(event `Frighten`
  (if (`self.Agrecive`)
    (`SceneComponent.SetVisibility` (`self.PlayerPostProces`) true false)
    (`KismetSystemLibrary.Delay` 0.5)
    (`SceneComponent.SetVisibility` (`self.PlayerPostProces`) false false)
    (`self.Frighten`)))

(event `Attac`
  (message `/Game/Bluprints/ThirdPerson/Blueprints/Interface/BPI_TakeDamage.TakeDamage` (`GameplayStatics.GetPlayerPawn` 0) 1)
  (bind _returnvalue (`PrimitiveComponent.CreateDynamicMaterialInstance` (`self.Sphere`) 0 "/Game/Bluprints/Enymy/shadow/Shadow/M_Fade.M_Fade" "None"))
  (bind _output_get (set `self.destroyMat` _returnvalue))
  (`MaterialInstanceDynamic.SetScalarParameterValue` _output_get "Param" -1.0)
  (`GameplayStatics.PlaySound2D` "/Game/Bluprints/Enymy/shadow/Shadow/hit-effekt-dlya-stsenyi-ujasa-quotkrik-robotaquot-32209__mp3cut_net_.hit-effekt-dlya-stsenyi-ujasa-quotkrik-robotaquot-32209__mp3cut_net_" 1.0 1.0 0.0 null null)
  (bind (_direction _newtrack_0) (`Timeline|Timeline`)
    (:`Update`
      (`MaterialInstanceDynamic.SetScalarParameterValue` (`self.destroyMat`) "Param" _newtrack_0))
    (:`Finished`
      (`SceneComponent.SetVisibility` (`self.PlayerPostProces`) false false)
      (`self.K2_DestroyActor`))))

(fn `UserConstructionScript`)