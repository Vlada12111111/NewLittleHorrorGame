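; Interactable window Blueprint that slides open and closed on alternate Interact calls.
; A FlipFlop plays or reverses a timeline that drives the relative location of MeshWindow01.
; Two cross-resetting DoOnce gates alternate drawer open and close sound cues, played at the world origin.
; BeginFocus and EndFocus toggle custom depth rendering on the window mesh.
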(event `/Game/Bluprints/MainCharacter/Blueprints/PlayerInterface/BPI_Interact.Interact`
  ;[1 1 1] Open Window
  (`/Engine/EditorBlueprintResources/StandardMacros.FlipFlop`
    (:`A`
      (`|ExecutionSequence`
        (:`then_0`
          (`/Engine/EditorBlueprintResources/StandardMacros.DoOnce` false :!label _label
            (:`Completed`
              (`GameplayStatics.PlaySoundAtLocation` "/Game/Asets/VHExterior/Audio/Cues/Cue_OpenDrawer.Cue_OpenDrawer" (0.0 0.0 0.0) (struct) 1.0 1.0 0.0 null null null null)
              (goto _label_3 :!via `Reset`))))
        (:`then_1`
          (bind (_direction _newtrack_0) (`Timeline|Timeline_0` :!label _label_2)
            (:`Update`
              (`SceneComponent.K2_SetRelativeLocation` (`self.Mesh_Window_01`) _newtrack_0 false false))))))
    (:`B`
      (`|ExecutionSequence`
        (:`then_0`
          (goto _label_2 :!via `Reverse`))
        (:`then_1`
          (`/Engine/EditorBlueprintResources/StandardMacros.DoOnce` false :!label _label_3
            (:`Completed`
              (`GameplayStatics.PlaySoundAtLocation` "/Game/Asets/VHExterior/Audio/Cues/Cue_CloseDrawer.Cue_CloseDrawer" (0.0 0.0 0.0) (struct) 1.0 1.0 0.0 null null null null)
              (goto _label :!via `Reset`))))))))

(fn `BeginFocus`
  (`PrimitiveComponent.SetRenderCustomDepth` (`self.Mesh_Window_01`) true))

(fn `EndFocus`
  (`PrimitiveComponent.SetRenderCustomDepth` (`self.Mesh_Window_01`) false))

(fn `UserConstructionScript`)