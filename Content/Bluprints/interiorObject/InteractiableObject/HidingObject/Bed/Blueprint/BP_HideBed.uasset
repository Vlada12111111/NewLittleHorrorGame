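; BP_HideBed is an interactable bed that lets the player hide under it and look around.
; Interact moves input from the pawn to the bed, and IA_Take hands it back.
; Both feed one FlipFlop that toggles IsHide, sends hide or unhide messages to the pawn and blends the view target between bed and pawn.
; While hidden, IA_Look rotates the bed's Camera within clamped yaw and pitch limits.
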(event `EnhancedInput|/Game/Bluprints/MainCharacter/Input/Actions/IA_Take`
  (params (ActionValue :type Boolean) (ElapsedSeconds :type "Float (double-precision)") (TriggeredSeconds :type "Float (double-precision)") (InputAction :type "InputAction Object Reference" :default "/Game/Bluprints/MainCharacter/Input/Actions/IA_Take.IA_Take"))
  (bind _returnvalue (`GameplayStatics.GetPlayerController` 0))
  (bind _returnvalue_2 (`GameplayStatics.GetPlayerPawn` 0))
  ;[1 1 1] Hide Under Bad
  (:`Triggered`
    (`self.EnableInput` (`GameplayStatics.GetPlayerPawn` 0) _returnvalue)
    (`self.DisableInput` _returnvalue)
    (`/Engine/EditorBlueprintResources/StandardMacros.FlipFlop` :!label _label
      (:`A`
        (set `self.IsHide` true)
        (message `/Game/Bluprints/MainCharacter/Blueprints/PlayerInterface/BPI_HideInterface.Hide` _returnvalue_2)
        (`PlayerController.SetViewTargetWithBlend` (`GameplayStatics.GetPlayerController` 0) self 0.5 "VTBlend_Linear" 0.0 false))
      (:`B`
        (set `self.IsHide` false)
        (message `/Game/Bluprints/MainCharacter/Blueprints/PlayerInterface/BPI_HideInterface.UnHide` _returnvalue_2)
        (`PlayerController.SetViewTargetWithBlend` (`GameplayStatics.GetPlayerController` 0) (`GameplayStatics.GetPlayerPawn` 0) 0.5 "VTBlend_Linear" 0.0 false)))))

(event `/Game/Bluprints/MainCharacter/Blueprints/PlayerInterface/BPI_Interact.Interact`
  (bind _returnvalue (`GameplayStatics.GetPlayerController` 0))
  ;[1 1 1] Hide Under Bad
  (`self.DisableInput` (`GameplayStatics.GetPlayerPawn` 0) _returnvalue)
  (`self.EnableInput` _returnvalue)
  (goto _label))

(event `EnhancedInput|/Game/Bluprints/MainCharacter/Input/Actions/IA_Look`
  (params (ActionValue :type "Vector2D Structure") (ElapsedSeconds :type "Float (double-precision)") (TriggeredSeconds :type "Float (double-precision)") (InputAction :type "InputAction Object Reference" :default "/Game/Bluprints/MainCharacter/Input/Actions/IA_Look.IA_Look"))
  ;[1 1 1] RotateCamera
  (:`Triggered`
    (if (`self.IsHide`)
      (`|ExecutionSequence`
        (:`then_0`
          ;;[1 1 1] calculate YAW
          (set `self.Yaw` (`KismetMathLibrary.FClamp` (+ (`self.Yaw`) ActionValue_X) -90.0 90.0)))
        (:`then_1`
          ;;[1 1 1] calculate Pitch
          (set `self.Pitch` (`KismetMathLibrary.FClamp` (+ (`self.Pitch`) (* ActionValue_Y -1.0)) -15.0 15.0)))
        (:`then_2`
          (`SceneComponent.K2_SetRelativeRotation` (`self.Camera`) (`KismetMathLibrary.MakeRotator` 0.0 (`self.Pitch`) (`self.Yaw`)) false false))))))

(fn `UserConstructionScript`)