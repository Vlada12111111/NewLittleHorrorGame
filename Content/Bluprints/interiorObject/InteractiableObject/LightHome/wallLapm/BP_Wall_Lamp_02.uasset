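; BP_Wall_Lamp_02 is an interactable wall lamp that the player switches on and off.
; Interact uses a FlipFlop to show or hide two point lights, first showing them, and plays a light sound cue at the world origin rather than at the lamp.
; BeginFocus and EndFocus toggle custom depth rendering on the Lamp component to mark focus.
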(event `/Game/Bluprints/MainCharacter/Blueprints/PlayerInterface/BPI_Interact.Interact`
  ;[1 1 1] On/Off Light
  (`/Engine/EditorBlueprintResources/StandardMacros.FlipFlop`
    (:`A`
      (`SceneComponent.SetVisibility` (`self.PointLight1`) true false)
      (`SceneComponent.SetVisibility` (`self.PointLight2`) true false))
    (:`B`
      (`SceneComponent.SetVisibility` (`self.PointLight1`) false false)
      (`SceneComponent.SetVisibility` (`self.PointLight2`) false false)))
  (`GameplayStatics.PlaySoundAtLocation` "/Game/Asets/VHExterior/Audio/Cues/Cue_Light.Cue_Light" (0.0 0.0 0.0) (struct) 1.0 1.0 0.0 null null null null))

(fn `BeginFocus`
  (`PrimitiveComponent.SetRenderCustomDepth` (`self.Lamp`) true))

(fn `EndFocus`
  (`PrimitiveComponent.SetRenderCustomDepth` (`self.Lamp`) false))

(fn `UserConstructionScript`)