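; BP_Door_01 is a swinging door that toggles open or closed when the player enters its trigger box, after a short delay, or when ChengeDoorStatus is called.
; A FlipFlop plays or reverses the Door timeline, which drives the yaw of MeshDoor02.
; Two cross-resetting DoOnce gates alternate the open and close sounds.
; BeginFocus and EndFocus toggle custom depth rendering on the door mesh.
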(event `self.Box.OnComponentBeginOverlap`
  (params (OverlappedComponent :type "PrimitiveComponent Object Reference") (OtherActor :type "Actor Object Reference") (OtherComp :type "PrimitiveComponent Object Reference") (OtherBodyIndex :type Integer) (bFromSweep :type Boolean) (SweepResult :type "HitResult Structure (by ref)"))
  ;[1 1 1] Open Door
  (if (== OtherActor (`GameplayStatics.GetPlayerPawn` 0))
    (`KismetSystemLibrary.Delay` 0.75)
    (`/Engine/EditorBlueprintResources/StandardMacros.FlipFlop` :!label _label
      (:`A`
        (`|ExecutionSequence`
          (:`then_0`
            (`/Engine/EditorBlueprintResources/StandardMacros.DoOnce` false :!label _label_2
              (:`Completed`
                (`GameplayStatics.PlaySoundAtLocation` "/Game/Asets/VHExterior/Audio/Cues/Cue_OpenDoor_01.Cue_OpenDoor_01" (0.0 0.0 0.0) (struct) 1.0 1.0 0.0 null null null null)
                (goto _label_4 :!via `Reset`))))
          (:`then_1`
            (bind (_direction _doorrotater) (`Timeline|Door` :!label _label_3)
              (:`Update`
                (`SceneComponent.K2_SetRelativeRotation` (`self.Mesh_Door_02`) (`KismetMathLibrary.MakeRotator` 0.0 0.0 _doorrotater) false false))))))
      (:`B`
        (`|ExecutionSequence`
          (:`then_0`
            (goto _label_3 :!via `Reverse`))
          (:`then_1`
            (`/Engine/EditorBlueprintResources/StandardMacros.DoOnce` false :!label _label_4
              (:`Completed`
                (`GameplayStatics.PlaySoundAtLocation` "/Game/Asets/VHExterior/Audio/Cues/Cue_CloseDoor_01.Cue_CloseDoor_01" (0.0 0.0 0.0) (struct) 1.0 1.0 0.0 null null null null)
                (goto _label_2 :!via `Reset`)))))))))

(event `/Game/Bluprints/MainCharacter/Blueprints/PlayerInterface/BPI_Interact.ChengeDoorStatus`
  ;[1 1 1] Open Door
  (goto _label))

(fn `BeginFocus`
  (`PrimitiveComponent.SetRenderCustomDepth` (`self.Mesh_Door_02`) true))

(fn `EndFocus`
  (`PrimitiveComponent.SetRenderCustomDepth` (`self.Mesh_Door_02`) false))

(fn `UserConstructionScript`)