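; Interactive wall lamp that can be switched on and off and highlights while focused.
; ChangeLiting flip-flops the visibility of two point lights, turning them off first, and plays a switch sound at world origin.
; OnFocus optionally enables custom depth on the lamp mesh for an outline and shows a prompt widget once through DoN.
; A retriggerable delay clears both and resets DoN shortly after focus calls stop.
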(event `/Game/Bluprints/LightHome/Candle/BPI_Candle.ChangeLiting`
  ;[1 1 1] On/Off Light
  (`/Engine/EditorBlueprintResources/StandardMacros.FlipFlop`
    (:`A`
      (`SceneComponent.SetVisibility` (`self.PointLight1`) false false)
      (`SceneComponent.SetVisibility` (`self.PointLight2`) false false))
    (:`B`
      (`SceneComponent.SetVisibility` (`self.PointLight1`) true false)
      (`SceneComponent.SetVisibility` (`self.PointLight2`) true false)))
  (`GameplayStatics.PlaySoundAtLocation` "/Game/Asets/VHExterior/Audio/Cues/Cue_Light.Cue_Light" (0.0 0.0 0.0) (struct) 1.0 1.0 0.0 null null null null))

(event `/Game/Asets/VHExterior/Blueprints/BP_InteractInterface.On Focus`
  ;[1 1 1] Outline
  (`|ExecutionSequence`
    (:`then_0`
      (if (`self.Outline on/off`)
        (`self.BeginFocus`))
      (set `self.TimeOutlineEnd` 0.1)
      (`KismetSystemLibrary.RetriggerableDelay` (`self.TimeOutlineEnd`))
      (`self.EndFocus`)
      (`Widget.RemoveFromParent` (stale _returnvalue))
      (`self.ResetOff`))
    (:`then_1`
      (`/Engine/EditorBlueprintResources/StandardMacros.Do N` 1 :!label _label
        (:`Exit`
          (bind _returnvalue (`|CreateWidget` "/Game/Asets/VHExterior/UMG/LightOff_Widget.LightOff_Widget_C"))
          (`UserWidget.AddToViewport` _returnvalue 0))))))

(event `ResetOff`
  ;[1 1 1] Outline
  (goto _label :!via `Reset`))

(fn `BeginFocus`
  (`PrimitiveComponent.SetRenderCustomDepth` (`self.Lamp`) true))

(fn `EndFocus`
  (`PrimitiveComponent.SetRenderCustomDepth` (`self.Lamp`) false))

(fn `UserConstructionScript`)