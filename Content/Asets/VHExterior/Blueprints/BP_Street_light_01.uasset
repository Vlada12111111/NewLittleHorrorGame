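; Interactable street light Blueprint with a focus outline and an on-screen widget, meant to switch its lamp on and off.
; OnInteract flip-flops between creating dynamic lamp materials, though both branches set the same emissive power, and plays a sound at world origin.
; OnFocus optionally enables custom depth and shows the widget once through a DoN gate.
; A short retriggerable delay clears both and resets the gate when focus calls stop.
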(event `/Game/Asets/VHExterior/Blueprints/BP_InteractInterface.OnInteract`
  ;[1 1 1] on/off Light
  (`/Engine/EditorBlueprintResources/StandardMacros.FlipFlop`
    (:`A`
      (bind _returnvalue (`PrimitiveComponent.CreateDynamicMaterialInstance` (`self.Lamp`) 1 "/Game/Asets/VHExterior/Materials/Instance/Tiling/Inst_Plastic_Glossy_03.Inst_Plastic_Glossy_03" "None"))
      (set `self.Dynamic material` _returnvalue)
      (`MaterialInstanceDynamic.SetScalarParameterValue` (`self.Dynamic material`) "PowerEmissive" 5.0))
    (:`B`
      (bind _returnvalue_2 (`PrimitiveComponent.CreateDynamicMaterialInstance` (`self.Lamp`) 1 "/Game/Asets/VHExterior/Materials/Instance/Tiling/Inst_Plastic_Glossy_03.Inst_Plastic_Glossy_03" "None"))
      (set `self.Dynamic material` _returnvalue_2)
      (`MaterialInstanceDynamic.SetScalarParameterValue` (`self.Dynamic material`) "PowerEmissive" 5.0)))
  (`GameplayStatics.PlaySoundAtLocation` "/Game/Asets/VHExterior/Audio/Cues/Cue_Light.Cue_Light" (0.0 0.0 0.0) (struct) 1.0 1.0 0.0 null null null null))

(event `/Game/Asets/VHExterior/Blueprints/BP_InteractInterface.On Focus`
  ;[1 1 1] Outline
  (`|ExecutionSequence`
    (:`then_0`
      (if (`self.Outline on/off`)
        (`self.BeginFocus`))
      (set `self.TimeOutlineEnd` 0.1)
      (`KismetSystemLibrary.RetriggerableDelay` (`self.TimeOutlineEnd`))
      (`self.EndFocus`)
      (`Widget.RemoveFromParent` (stale _returnvalue))
      (`self.ResetOff`))
    (:`then_1`
      (`/Engine/EditorBlueprintResources/StandardMacros.Do N` 1 :!label _label
        (:`Exit`
          (bind _returnvalue (`|CreateWidget` "/Game/Asets/VHExterior/UMG/LightOff_Widget.LightOff_Widget_C"))
          (`UserWidget.AddToViewport` _returnvalue 0))))))

(event `ResetOff`
  ;[1 1 1] Outline
  (goto _label :!via `Reset`))

(fn `BeginFocus`
  (`PrimitiveComponent.SetRenderCustomDepth` (`self.Lamp`) true))

(fn `EndFocus`
  (`PrimitiveComponent.SetRenderCustomDepth` (`self.Lamp`) false))

(fn `UserConstructionScript`)