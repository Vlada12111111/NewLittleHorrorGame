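; BP_Picture is an interactable picture that the player can focus on and toggle a zoomed view of.
; Interacting flip-flops the view target between the picture and the character with a blend, zeroing walk speed while zoomed and setting it back on exit.
; Focus optionally outlines the mesh through custom depth and shows a Scale widget once through a DoN gate.
; A short retriggerable delay detects lost focus, then clears both and resets the gate.
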(event `/Game/Asets/VHExterior/Blueprints/BP_InteractInterface.OnInteract`
  (`/Engine/EditorBlueprintResources/StandardMacros.FlipFlop`
    (:`A`
      ;[1 1 1] ZoomIn
      (`PlayerController.SetViewTargetWithBlend` (`GameplayStatics.GetPlayerController` 0) self 1.0 "VTBlend_Linear" 0.0 true)
      (set `CharacterMovementComponent.MaxWalkSpeed` 0.0 (`Character.CharacterMovement` (`GameplayStatics.GetPlayerCharacter` 0))))
    (:`B`
      ;[1 1 1] ZoomOut
      (`PlayerController.SetViewTargetWithBlend` (`GameplayStatics.GetPlayerController` 0) (`GameplayStatics.GetPlayerCharacter` 0) 1.0 "VTBlend_Linear" 0.0 true)
      (set `CharacterMovementComponent.MaxWalkSpeed` 150.0 (`Character.CharacterMovement` (`GameplayStatics.GetPlayerCharacter` 0))))))

(event `/Game/Asets/VHExterior/Blueprints/BP_InteractInterface.On Focus`
  ;[1 1 1] Outline
  (`|ExecutionSequence`
    (:`then_0`
      (if (`self.Outline on/off`)
        (`self.BeginFocus`))
      (set `self.TimeOutlineEnd` 0.1)
      (`KismetSystemLibrary.RetriggerableDelay` (`self.TimeOutlineEnd`))
      (`self.EndFocus`)
      (`Widget.RemoveFromParent` (stale _returnvalue))
      (`self.Reset` false))
    (:`then_1`
      (`/Engine/EditorBlueprintResources/StandardMacros.Do N` 1 :!label _label
        (:`Exit`
          (bind _returnvalue (`|CreateWidget` "/Game/Asets/VHExterior/UMG/Scale_Widget.Scale_Widget_C"))
          (`UserWidget.AddToViewport` _returnvalue 0))))))

(event `Reset`
  (params (NewParam :type Boolean))
  ;[1 1 1] Outline
  (goto _label :!via `Reset`))

(fn `BeginFocus`
  (`PrimitiveComponent.SetRenderCustomDepth` (`self.Mesh_Picture`) true))

(fn `EndFocus`
  (`PrimitiveComponent.SetRenderCustomDepth` (`self.Mesh_Picture`) false))

(fn `UserConstructionScript`)